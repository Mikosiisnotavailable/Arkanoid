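; BP_ball is the ball actor for an Arkanoid test game.
; Each tick it moves its sphere component with a sweep along a direction scaled by speed, using only X and Y.
; On a blocking hit it reflects the direction about the hit normal and raises the speed by a set increment up to a fixed cap.
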(event `self.ReceiveTick`
  (params (DeltaSeconds :type "Float (single-precision)"))
  (bind (_returnvalue_x _returnvalue_y) (`KismetMathLibrary.BreakVector` (* (`self.Direction`) (* DeltaSeconds (`self.speed`)))))
  (bind _sweephitresult (`SceneComponent.K2_AddWorldOffset` (`self.Sphere`) (`KismetMathLibrary.MakeVector` _returnvalue_x _returnvalue_y) true false))
  (bind (_bblockinghit _binitialoverlap _time _distance _location _impactpoint _normal) (`GameplayStatics.BreakHitResult` _sweephitresult))
  (if _bblockinghit
    (set `self.Direction` (`KismetMathLibrary.GetReflectionVector` (`self.Direction`) _normal))
    (set `self.speed` (`KismetMathLibrary.FMin` (+ (`self.speed`) (`self.Added Speed`)) 4000.0))))

(fn `UserConstructionScript`)