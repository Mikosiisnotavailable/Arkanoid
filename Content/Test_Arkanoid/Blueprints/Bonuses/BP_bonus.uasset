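; BP_bonus is a bonus Blueprint for an Arkanoid test game that moves along the world X axis.
; Its construction script randomly picks one of two bonus types and shows the enum name on a text render component.
; Each tick offsets the Bon component by the X part of Direction scaled by Speed and delta time.
; It contains no overlap or pickup logic.
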(event `self.ReceiveTick`
  (params (DeltaSeconds :type "Float (single-precision)"))
  (bind _returnvalue_x (`KismetMathLibrary.BreakVector` (* (`self.Direction`) (* DeltaSeconds (`self.speed`)))))
  (`SceneComponent.K2_AddWorldOffset` (`self.bon `) (`KismetMathLibrary.MakeVector` _returnvalue_x) false false))

(fn `UserConstructionScript`
  (set `self.BonType` (select `int` (`KismetMathLibrary.RandomIntegerInRange` 0 1) :`0` "NewEnumerator0" :`1` "NewEnumerator1" :!type "/Game/Test_Arkanoid/Blueprints/Bonuses/E_Bon_type Enum"))
  (`TextRenderComponent.K2_SetText` (`self.TextRender`) (`KismetTextLibrary.Conv_StringToText` (`|GetEnumeratorNameAsString` (`self.BonType`)))))