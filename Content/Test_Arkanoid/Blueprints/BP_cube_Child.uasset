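; BP_cube_Child is an Arkanoid cube variant, derived from a parent Blueprint, that can drop a bonus when destroyed.
; BallHit and the construction script only forward to the parent.
; On BeginPlay it binds SpawnBon to its own OnDestroyed, which has a one-in-seven chance to spawn a BP_bonus at the cube's location with a fixed rotation.
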(event `self.BallHit`
  (`parent.BallHit`))

(event `self.ReceiveBeginPlay`
  (add `self.OnDestroyed` (delegate `SpawnBon`)))

(event `SpawnBon` :!signature `self.OnDestroyed`
  (params (DestroyedActor :type "Actor Object Reference"))
  (if (== (`KismetMathLibrary.RandomIntegerInRange` 1 7) 7)
    (`|SpawnActorFromClass` "/Game/Test_Arkanoid/Blueprints/Bonuses/BP_bonus.BP_bonus_C" (`KismetMathLibrary.MakeTransform` (`self.K2_GetActorLocation`) (struct :`Pitch` 90.0)) "AlwaysSpawn" "OverrideRootScale" null null)))

(fn `UserConstructionScript`
  (`parent.UserConstructionScript`))