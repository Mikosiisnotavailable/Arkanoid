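; BP_level_gen is an Arkanoid level generator that spawns the cube grid and detects when it is cleared.
; The construction script builds an X-by-Y static mesh preview, which BeginPlay destroys and replaces with BP_cube_Child actors in a randomly sized, padded grid.
; Each cube's death event feeds DeathCube, which adds score to BP_my_pawn and fires AllCubesDied once the death count reaches the spawned total.
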(event `self.ReceiveBeginPlay`
  (bind (_returnvalue_x _returnvalue_y _returnvalue_z) (`KismetMathLibrary.BreakVector` (`self.K2_GetActorLocation`)))
  (`|ExecutionSequence`
    (:`then_0`
      (bind _returnvalue (`GameplayStatics.GetActorOfClass` "/Game/Test_Arkanoid/Blueprints/Core/pawn_and_cntrl/BP_my_pawn.BP_my_pawn_C"))
      (set `self.MyPawn` _returnvalue))
    (:`then_1`
      (for _array_element (`self.Preview`)
        (`ActorComponent.K2_DestroyComponent` _array_element))
      (for _index (range (+ (`KismetMathLibrary.RandomIntegerInRange` (`self.x`) 5) 1))
        (for _index_2 (range (+ (`KismetMathLibrary.RandomIntegerInRange` (`self.y`) 7) 1))
          (bind _returnvalue_2 (`|SpawnActorFromClass` "/Game/Test_Arkanoid/Blueprints/BP_cube_Child.BP_cube_Child_C" (`KismetMathLibrary.MakeTransform` (`KismetMathLibrary.MakeVector` (+ (`KismetMathLibrary.Conv_IntToDouble` (* _index (`self.padding`))) _returnvalue_x) (+ (* _index_2 (`self.padding`)) _returnvalue_y) _returnvalue_z)) "Undefined" "OverrideRootScale" null null))
          (`KismetArrayLibrary.Array_Add` (`self.CubeAmmount`) _returnvalue_2)))
      (bind _amountcubes (`self.Get_For_Win`))
      (set `self.Amount Cubes for win` _amountcubes)
      (for _array_element_2 (`self.CubeAmmount`)
        (add `/Game/Test_Arkanoid/Blueprints/BP_cube_Parent.Cube Dead` _array_element_2 (delegate `DeathCube`))))))

(event `DeathCube`
  (params (Score :type Integer))
  (`/Game/Test_Arkanoid/Blueprints/Core/pawn_and_cntrl/BP_my_pawn.Added Score` (`self.MyPawn`) Score)
  (`/Engine/EditorBlueprintResources/StandardMacros.IncrementInt` (`self.DeadCubes`)
    (:`  `
      (if (>= (`self.DeadCubes`) (`self.Amount Cubes for win`))
        (`KismetSystemLibrary.PrintText` "")
        (`self.AllCubesDied`)))))

(fn `Get_For_Win`
  (returns (AmountCubes :type Integer))
  (return (`KismetArrayLibrary.Array_Length` (`self.CubeAmmount`))))

(fn `UserConstructionScript`
  (for _index (range (+ (`self.x`) 1))
    (for _index_2 (range (+ (`self.y`) 1))
      (bind _returnvalue (`AddComponent|NODE_AddStaticMeshComponent-0` :`RelativeTransform` (`KismetMathLibrary.MakeTransform` (`KismetMathLibrary.MakeVector` (`KismetMathLibrary.Conv_IntToDouble` (* _index (`self.padding`))) (`KismetMathLibrary.Conv_IntToDouble` (* _index_2 (`self.padding`)))))))
      (`KismetArrayLibrary.Array_Add` (`self.Preview`) _returnvalue))))