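; Player controller for an Arkanoid test game that moves the possessed pawn sideways and triggers its spawner from input.
; On BeginPlay it creates the HUD widget and listens for the level generator's all-cubes-died event.
; That event and the pawn's game-end event both call Endgame, which hides the HUD, shows WBP_Win and switches to UI-only input with a cursor.
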(event `self.ReceiveBeginPlay`
  (`|ExecutionSequence`
    (:`then_0`
      (`WidgetBlueprintLibrary.SetInputMode_GameOnly` self)
      (bind _returnvalue (`|CreateWidget` "/Game/Test_Arkanoid/UI/WBP_Hud.WBP_Hud_C" self))
      (`UserWidget.AddToViewport` _returnvalue 0)
      (set `self.lives` _returnvalue))
    (:`then_1`
      (bind _returnvalue_2 (`GameplayStatics.GetActorOfClass` "/Game/Test_Arkanoid/Blueprints/BP_level_gen.BP_level_gen_C"))
      (add `/Game/Test_Arkanoid/Blueprints/BP_level_gen.AllCubesDied` _returnvalue_2 (delegate `Endgame`)))))

(event `Endgame`
  (`Widget.SetVisibility` (`self.lives`) "Collapsed")
  (bind _returnvalue (`|CreateWidget` "/Game/Test_Arkanoid/UI/WBP_Win.WBP_Win_C" self))
  (`UserWidget.AddToViewport` _returnvalue 0)
  (`WidgetBlueprintLibrary.SetInputMode_UIOnlyEx` self _returnvalue "LockOnCapture")
  (set `self.bShowMouseCursor` true))

(event `self.ReceivePossess`
  (params (PossessedPawn :type "Pawn Object Reference"))
  (bind _asbp_my_pawn (cast `/Game/Test_Arkanoid/Blueprints/Core/pawn_and_cntrl/BP_my_pawn` PossessedPawn))
  (bind _output_get (set `self.As BP My Pawn` _asbp_my_pawn))
  (add `/Game/Test_Arkanoid/Blueprints/Core/pawn_and_cntrl/BP_my_pawn.gameend` _output_get (delegate `Endgame`)))

(event `InputAxis|AD`
  (params (AxisValue :type "Float (single-precision)"))
  (`self.K2_AddActorWorldOffset` (`self.As BP My Pawn`) (`KismetMathLibrary.MakeVector` 0.0 (* AxisValue (`GameplayStatics.GetWorldDeltaSeconds`) (`self.speed`))) true false))

(event `InputAction|spawner`
  (params (Key :type "Key Structure"))
  (:`Pressed`
    (`/Game/Test_Arkanoid/Blueprints/Core/pawn_and_cntrl/BP_my_pawn.Spawner` (`self.As BP My Pawn`))))

(fn `UserConstructionScript`)